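; Audio-reactive spotlight actor that plays a sound and pulses light intensity and outer cone angle with that sound's loudness.
; Each playback-percent callback converts progress to seconds and samples the pre-analysed (non-real-time) normalized loudness for the chosen channel, scaled by per-light multipliers.
; The construction script caches duration and builds an onset-based, remapped Constant-Q spectrum, which the light logic never uses; the instance setup loop is empty.
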(event Custom|OnAudioPlaybackPercent_Event
  (params (PlayingSoundWave :type Sound%20Wave%20Object%20Reference) (PlaybackPercent :type Float%20%28single-precision%29))
  (bind _spotlight (Variables|Default|GetSpotLight))
  (bind _loudnessanalyser__preruntime_ (Variables|Default|GetLoudnessAnalyser%20%28PreRuntime%29))
  (bind _channel__0_or_1_ (Variables|Default|GetChannel%20%280%20or%201%29))
  (bind _duration (Variables|Default|GetDuration))
  (bind _returnvalue (* PlaybackPercent _duration))
  (bind _outloudness (Class|LoudnessNRT|GetNormalizedChannelLoudnessatTime _loudnessanalyser__preruntime_ _returnvalue _channel__0_or_1_))
  (Rendering|Components|Light|SetIntensity _spotlight (* _outloudness (Variables|Default|GetLightIntenstityUnitsL1)))
  (Rendering|Lighting|SetOuterConeAngle _spotlight (* _outloudness (Variables|Default|GetOuterConeAngleMultiplierL1)))
  (Rendering|Lighting|SetInnerConeAngle _spotlight (Variables|Default|GetInnerConeAngleMultiplierL1)))

(event EventBeginPlay
  (bind _inputaudio (Variables|Default|GetInputAudio))
  (Audio|Components|Audio|AdjustVolume (Variables|Default|GetInputAudio) 0.0 (Variables|Default|GetVolume%20%28%200%20to%201%29) "Linear" :!class /Script/Engine.AudioComponent)
  (Rendering|Lighting|SetAttenuationRadius (Variables|Default|GetSpotLight) (Variables|Default|GetAttenuationRadiusL1))
  (Rendering|Components|Light|SetLightColor (Variables|Default|GetSpotLight) (Variables|Default|GetColourL1) true)
  (Audio|Components|Audio|SetSound _inputaudio (Variables|Default|GetSoundWaveToAnalyse))
  (EventDispatchers|AssignOnAudioPlaybackPercent (Variables|Default|GetInputAudio) (delegate Custom|OnAudioPlaybackPercent_Event))
  (Audio|Components|Audio|Play _inputaudio 0.0))

(fn ConstructionScript
  (bind _loudnessanalyser__preruntime_ (Variables|Default|GetLoudnessAnalyser%20%28PreRuntime%29))
  (bind _sound (Variables|/Script/AudioAnalyzer.AudioAnalyzerNRT|GetSound _loudnessanalyser__preruntime_))
  (CallFunction|SetupInstances 150)
  (Audio|Components|Audio|SetSound (Variables|Default|GetInputAudio) _sound)
  (Variables|Default|SetDuration (Variables|/Script/Engine.SoundBase|GetDuration _sound))
  (Variables|Default|SetOut%20Onset%20Timestamps (.OutOnsetTimestamps (Class|OnsetNRT|GetChannelOnsetsBetweenTimes (Variables|Default|GetEventAnalyser) 0.0 (Variables|/Script/Engine.SoundBase|GetDuration _sound))))
  (bind _output_get (Utilities|GetFreqMax (.OutOnsetTimestamps (Class|OnsetNRT|GetChannelOnsetsBetweenTimes (Variables|Default|GetEventAnalyser) 0.0 (Variables|/Script/Engine.SoundBase|GetDuration _sound))) (Variables|Default|GetFreqAnalyser))
    (:Completed
      (bind _output_get_2 (Variables|Default|SetFreqMax _output_get))
      (bind _output_get_3 (CallFunction|RemapFreqResponse (Class|ConstantQNRT|GetChannelConstantQatTime (Variables|Default|GetFreqAnalyser) (Variables|Default|GetFreqTimeStamp)) -6e+01 _output_get_2))
      (Variables|Default|SetOut%20Constant%20Q _output_get_3))))

(fn SetupInstances
  (params (Spacing :type Integer))
  (for _index (range 0 (Variables|/Script/AudioSynesthesia.ConstantQNRTSettings|GetNumBands (Variables|/Script/AudioSynesthesia.ConstantQNRT|GetSettings (Variables|Default|GetFreqAnalyser))))
    _)
  (return))

(fn UpdateInstances
  (params (InSeconds :type Float%20%28single-precision%29) (Height%20Scale :type Float%20%28double-precision%29))
  (CallFunction|RemapFreqResponse (Class|ConstantQNRT|GetChannelConstantQatTime (Variables|Default|GetFreqAnalyser) InSeconds) -6e+01 (Variables|Default|GetFreqMax)))

(fn RemapFreqResponse
  (params (Array :type Array%20of%20Floats%20%28single-precision%29) (InRangeA :type Float%20%28double-precision%29) (InRangeB :type Float%20%28double-precision%29))
  (bind _newlocalvar_3 (LocalVariables|GetNewLocalVar_3))
  (for _array_element Array
    (Utilities|Array|Add _newlocalvar_3 (Math|Float|MapRangeClamped _array_element InRangeA InRangeB 0.0 1.0)))
  (return _newlocalvar_3))